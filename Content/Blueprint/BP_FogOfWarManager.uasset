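; Fog of war manager Blueprint that displays the fog texture as a post-process effect.
; Construction creates a dynamic instance of the fog material and adds it to the PostProcess component as a blendable.
; OnFowTextureUpdated feeds the current and previous textures into that material and resets its Blend parameter.
; Tick ramps Blend back to one over about a tenth of a second, smoothing transitions between fog updates.
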(event EventBeginPlay)

(event Collision|EventActorBeginOverlap
  (params (OtherActor :type Actor%20Object%20Reference)))

(event EventTick
  (params (DeltaSeconds :type Float%20%28single-precision%29))
  (bind _self self)
  (if (< (Variables|Default|GetFowTextureBlend) 1.0)
    (bind _output_get (Variables|Default|SetFowTextureBlend (Math|Float|Clamp(Float) (+ (* DeltaSeconds 1e+01) (Variables|Default|GetFowTextureBlend)))))
    (Rendering|Material|SetScalarParameterValue (Variables|Default|GetDynamicMat) "Blend" _output_get :!class /Script/Engine.MaterialInstanceDynamic)
    (elif (not (Variables|Default|GetbIsDoneBlending _self))
      (Variables|Default|SetbIsDoneBlending _self true))))

(event EventOnFowTextureUpdated
  (params (currentTexture :type Texture%202D%20Object%20Reference) (lastTexture :type Texture%202D%20Object%20Reference))
  (bind _dynamicmat (Variables|Default|GetDynamicMat))
  (Rendering|Material|SetTextureParameterValue _dynamicmat "FowTexture" currentTexture)
  (Rendering|Material|SetTextureParameterValue _dynamicmat "LastFowTexture" lastTexture)
  (Rendering|Material|SetScalarParameterValue _dynamicmat "Blend" 0.0 :!class /Script/Engine.MaterialInstanceDynamic)
  (Variables|Default|SetFowTextureBlend 0.0))

(fn ConstructionScript
  (bind _returnvalue (Rendering|Material|CreateDynamicMaterialInstance "/Game/Material/Fow/PP_Fow_Mat.PP_Fow_Mat" :!class /Script/Engine.KismetMaterialLibrary))
  (Variables|Default|SetDynamicMat _returnvalue)
  (Rendering|AddorUpdateBlendable (Variables|Default|GetPostProcess) _returnvalue 1.0 :!class /Script/Engine.PostProcessComponent))